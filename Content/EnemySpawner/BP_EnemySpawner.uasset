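; BP_EnemySpawner is a spawner that periodically creates BP_EnemyPawn enemies at its own location, up to a population cap.
; BeginPlay starts a looping EnemyRate timer calling SpawnItem, which uses SpawnAIFromClass while the world-wide pawn count is below MaxEnemies.
; AttemptToSpawn and debug GetEnemyCount are not called here.
; SpawnEnemy1 is empty, and an old random-pick SpawnActor path is disconnected.
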(event EventBeginPlay
  (Utilities|Time|SetTimerbyFunctionName 0 "SpawnItem" (Math|Conversions|ToFloat(Integer) (Variables|Default|GetEnemyRate)) true))

(fn ConstructionScript)

(fn SpawnEnemy1)

(fn AttempttoSpawn
  (Utilities|IsValid (Variables|Default|GetCurrentEnemy)
    (:Is%20Valid
      (Development|PrintString "Enemy already Spawned"))
    (:Is%20Not%20Valid
      (CallFunction|SpawnItem))))

(fn SpawnItem
  (bind _outactors (Actor|GetAllActorsOfClass "/Game/EnemySpawner/BP_EnemyPawn.BP_EnemyPawn_C"))
  (Math|Integer|CompareInt (Utilities|Array|Length _outactors) (Variables|Default|GetMaxEnemies)
    (:<
      (AI|SpawnAIFromClass "/Game/EnemySpawner/BP_EnemyPawn.BP_EnemyPawn_C" 0 (Transformation|GetActorLocation) (Transformation|GetActorRotation) false))))

(fn GetEnemyCount
  (bind _outactors (Actor|GetAllActorsOfClass "/Game/EnemySpawner/BP_EnemyPawn.BP_EnemyPawn_C"))
  (Development|PrintString (Utilities|String|ToString(Integer) (Utilities|Array|Length _outactors))))